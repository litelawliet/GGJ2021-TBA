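; Enemy AI character that patrols a looping point path, fires ghost projectiles at the player and is destroyed by a single hit.
; FindDest advances through PatrolPath, wrapping to the start, and writes the next point to the Blackboard.
; FireProjectile faces the cached player target, re-fetching it if invalid, and leads the shot using player velocity and distance.
; Tick bobs the static mesh on a sine wave around its starting offset.
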(event `self.ReceiveBeginPlay`
  (set `self.CurDest` (`|GetArrayItem` (`self.PatrolPath`)))
  (set `self.Arrived` true)
  (set `self.DestBBRef` "DestActor")
  (bind _asthird_person_character (cast `/Game/ThirdPersonBP/Blueprints/ThirdPersonCharacter` (`GameplayStatics.GetPlayerCharacter` 0)))
  (set `self.Target` _asthird_person_character)
  (set `self.MeshLocation` (`SceneComponent.RelativeLocation` (`self.StaticMesh`))))

(event `FindDest`
  (bind _patrolpath (`self.PatrolPath`))
  (bind _patrolpath_2 (`self.PatrolPath`))
  (bind _returnvalue (+ (`KismetArrayLibrary.Array_Find` _patrolpath (`self.CurDest`)) 1))
  (if (> _returnvalue (- (`KismetArrayLibrary.Array_Length` _patrolpath) 1))
    ;[1 1 1] Set new destination depending on fetched index
    (set `self.CurDest` (`|GetArrayItem` _patrolpath_2))
    (else
      (set `self.CurDest` (`|GetArrayItem` _patrolpath_2 _returnvalue))))
  (`BlackboardComponent.SetValueAsObject` (`AIBlueprintHelperLibrary.GetBlackboard` null) (`self.DestBBRef`) (`self.CurDest`)))

(event `ReceiveDmg`
  ;[1 1 1] Receive damage from player projectile
  (`self.K2_DestroyActor`))

(event `self.ReceiveTick`
  (params (DeltaSeconds :type "Float (single-precision)"))
  (set `self.BobbingCycle` (mod (+ (`self.BobbingCycle`) (/ (* (`GameplayStatics.GetWorldDeltaSeconds`) 360.0) (`self.BobbingPeriod`))) 360.0))
  (`SceneComponent.K2_SetRelativeLocation` (`self.StaticMesh`) (+ (`self.MeshLocation`) (`KismetMathLibrary.MakeVector` 0.0 0.0 (* (`self.BobbingAmplitude`) (`KismetMathLibrary.DegSin` (`self.BobbingCycle`))))) false false))

(fn `FireProjectile`
  (bind _target (`self.Target`))
  (bind _returnvalue (`SceneComponent.K2_GetComponentLocation` (`self.ProjectileSpawner`)))
  (bind _returnvalue_2 (`self.K2_GetActorLocation` _target))
  (if (not (`KismetSystemLibrary.IsValid` (`self.Target`)))
    (bind _asthird_person_character (cast `/Game/ThirdPersonBP/Blueprints/ThirdPersonCharacter` (`GameplayStatics.GetPlayerCharacter` 0)))
    (set `self.Target` _asthird_person_character))
  ;[1 1 1] Rotate agent to face player
  (`self.K2_SetActorRotation` (`KismetMathLibrary.FindLookAtRotation` (`self.K2_GetActorLocation` self) _returnvalue_2))
  (`|SpawnActorFromClass` "/Game/AI/GhostPrjectile_BP.GhostPrjectile_BP_C" (`KismetMathLibrary.MakeTransform` _returnvalue (`KismetMathLibrary.FindLookAtRotation` _returnvalue (+ _returnvalue_2 (* (`self.GetVelocity` _target) (/ (`self.GetDistanceTo` self _target) 1500.0)))) (0.5 0.5 0.5)) "Undefined" "OverrideRootScale" null null))

(fn `UserConstructionScript`)