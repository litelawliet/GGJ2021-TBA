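; Ghost projectile actor that costs the third-person player character a heart on contact.
; BeginPlay sets the projectile movement's initial speed from Speed, then destroys the actor once ProjectileLifetime elapses.
; Overlapping the player calls LoseHeart on its StaminaHealthController and destroys the projectile immediately.
; Other overlaps only attempt a static mesh component cast, with no further effect.
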(event `self.ReceiveBeginPlay`
  ;[1 1 1] Setup initial speed and lifetime
  (set `ProjectileMovementComponent.InitialSpeed` (`self.Speed`) (`self.ProjectileMovement`))
  (`KismetSystemLibrary.Delay` (`self.ProjectileLifetime`))
  (`self.K2_DestroyActor` :!label _label))

(event `self.ReceiveActorBeginOverlap`
  (params (OtherActor :type "Actor Object Reference"))
  ;[1 1 1] Collide With Player
  (bind _asthird_person_character (cast `/Game/ThirdPersonBP/Blueprints/ThirdPersonCharacter` OtherActor)
    (:`then`
      (`/Game/ThirdPersonBP/Blueprints/StaminaHealthController.Lose Heart` (`/Game/ThirdPersonBP/Blueprints/ThirdPersonCharacter.StaminaHealthController` _asthird_person_character))
      (goto _label))
    (:`CastFailed`
      (cast `StaticMeshComponent` (`self.GetComponentByClass` OtherActor "/Script/Engine.StaticMeshComponent")))))

(fn `UserConstructionScript`)