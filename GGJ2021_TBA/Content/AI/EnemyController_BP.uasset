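; AI controller for the enemy character that drives it with a behavior tree and reacts to seeing the player.
; On possessing an EnemyCharacter_BP it stores the pawn and runs AITree_BT.
; AI perception updates for the third-person character write the sensed state and the player reference to blackboard keys, whose names are set at BeginPlay.
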(event `self.AIPerception.OnTargetPerceptionUpdated`
  (params (Actor :type "Actor Object Reference") (Stimulus :type "AIStimulus Structure"))
  (bind _returnvalue (`AIBlueprintHelperLibrary.GetBlackboard` null))
  (cast `/Game/ThirdPersonBP/Blueprints/ThirdPersonCharacter` Actor)
  (`BlackboardComponent.SetValueAsBool` _returnvalue (`self.LOSBBRef`) (`.bSuccessfullySensed` (break `AIStimulus` Stimulus)))
  (`BlackboardComponent.SetValueAsObject` _returnvalue (`self.PlayerBBRef`) "/Game/ThirdPersonBP/Blueprints/ThirdPersonCharacter.ThirdPersonCharacter"))

(event `self.ReceivePossess`
  (params (PossessedPawn :type "Pawn Object Reference"))
  (bind _asenemy_character_bp (cast `/Game/AI/EnemyCharacter_BP` PossessedPawn))
  (set `self.Enemy` _asenemy_character_bp)
  (`self.RunBehaviorTree` "/Game/AI/AITree_BT.AITree_BT"))

(event `self.ReceiveBeginPlay`
  (set `self.PlayerBBRef` "PlayerActor")
  (set `self.LOSBBRef` "CanSeePlayer"))

(fn `UserConstructionScript`)