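; PatrolPoint_BP is a patrol point actor that builds a list of nearby patrol points at BeginPlay.
; It scans all PatrolPoint_BP actors and adds those within the NavBubble sphere's radius to NextPoints, comparing squared distances rather than using overlaps.
; The scan does not exclude the point itself, so each point also lists itself.
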(event `self.ReceiveBeginPlay`
  (bind _outactors (`GameplayStatics.GetAllActorsOfClass` "PatrolPoint_BP_C"))
  (for _array_element _outactors
    (if (<= (`KismetMathLibrary.Vector_DistanceSquared` (`self.K2_GetActorLocation` _array_element) (`self.K2_GetActorLocation` self)) (`KismetMathLibrary.Square` (`SphereComponent.SphereRadius` (`self.NavBubble`))))
      (`KismetArrayLibrary.Array_Add` (`self.NextPoints`) _array_element))))

(fn `UserConstructionScript`)